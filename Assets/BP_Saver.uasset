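; BP_Saver is an actor that stores a DBRecord, including a MOTD, as persistent game data through its ActorPersistence component.
; On BeginPlay it ensures a unique ID, marking itself dirty if newly created, and binds a data-loaded callback.
; DBWrite replaces the record and marks it dirty, while DBRead uses the first existing saver or spawns one.
; Debug prints report binding, loading and the MOTD on a delayed tick.
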(event Custom|DataLoaded
  (Development|PrintString (Utilities|String|Append "Data Loaded (MOTD):" (Utilities|Struct|BreakDB_Saver_Record (Variables|Default|GetDBRecord)))))

(event Custom|DBWrite
  (params (DBRecord :type DB%20Saver%20Record%20Structure))
  (Variables|Default|SetDBRecord DBRecord)
  (Class|PersistenceComponent|SetDirty (Variables|Default|GetActorPersistence) true))

(event EventBeginPlay
  (bind _actorpersistence (Variables|Default|GetActorPersistence))
  (if (Class|DreamworldBlueprints|IsValidID (Class|PersistenceComponent|GetUniqueID (Variables|Default|GetActorPersistence)))
    (EventDispatchers|BindEventtoOnSignalDataLoaded (Variables|Default|GetActorPersistence) (delegate Custom|DataLoaded))
    (Development|PrintString "Bind ID Exists")
    (else
      (bind _returnvalue (Class|UniqueID|GenerateUniqueID))
      (Class|DreamworldBlueprints|SetUniqueID self _returnvalue)
      (Class|PersistenceComponent|SetDirty _actorpersistence true)
      (EventDispatchers|BindEventtoOnSignalDataLoaded _actorpersistence (delegate Custom|DataLoaded))
      (Development|PrintString "Bind Created new UID"))))

(event Collision|EventActorBeginOverlap
  (params (OtherActor :type Actor%20Object%20Reference)))

(event EventTick
  (params (DeltaSeconds :type Float%20%28single-precision%29))
  (Utilities|FlowControl|Delay 2.0)
  (Development|PrintString (Utilities|String|Append "Tick:" (Utilities|Struct|BreakDB_Saver_Record (Variables|Default|GetDBRecord))) true true "(R=0.082484,G=1.000000,B=0.000000,A=1.000000)"))

(fn ConstructionScript)

(fn DBRead
  (bind _outactors (Actor|GetAllActorsOfClass "BP_Saver_C"))
  (if (Utilities|IsValid (Utilities|Array|Get(acopy) _outactors))
    (return (Variables|BP_Saver_C|GetDBRecord (Utilities|Array|Get(acopy) _outactors)))
    (else
      (bind _returnvalue (Game|SpawnActorfromClass "BP_Saver_C" (Math|Transform|MakeTransform "0, 0, 0") "Undefined" 0 (Game|GetPlayerCharacter 0)))
      (return (Variables|BP_Saver_C|GetDBRecord _returnvalue)))))